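; Player character Blueprint for a mouse-driven medicine (药品) scene, with WASD movement and right-mouse-held camera look.
; A looping timer traces from the camera along the cursor direction and sends SeeItemMessage to the hit actor to show medicine names.
; 背包物品添加 appends medicine info to the inventory array, storing its index as its ID.
; Left-click physics grab is unfinished: it traces from screen center, but grab and move logic are disconnected.
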(event Custom|药品名称可视化
  ;[1 1 1] 鼠标发射射线检测药品，显示名称
  (bind _returnvalue (Utilities|Time|SetTimerbyEvent (delegate Custom|发射射线) (Variables|Default|Get射线发射率) true))
  (Variables|Default|Set射线时间 _returnvalue))

(event Custom|发射射线
  (bind _camera (Variables|Default|GetCamera))
  (bind _returnvalue (Transformation|GetWorldLocation _camera))
  ;[1 1 1] 鼠标发射射线检测药品，显示名称
  (bind (_outhit _returnvalue_2) (Collision|LineTraceByChannel _returnvalue (+ _returnvalue (* (.WorldDirection (Game|Player|ConvertMouseLocationToWorldSpace (Game|GetPlayerController 0))) (Variables|Default|Get射线长度))) "TraceTypeQuery1" false 0 "None"))
  (if _returnvalue_2
    (Class|SeeItem|SeeItem(Message) (.HitActor (Collision|BreakHitResult _outhit)))))

(event EventTick
  (params (DeltaSeconds :type Float%20%28single-precision%29)))

(event EventBeginPlay
  (bind _returnvalue (Game|GetPlayerController 0))
  (CallFunction|药品名称可视化)
  (Variables|/Script/Engine.PlayerController|SetbShowMouseCursor _returnvalue true)
  (Variables|/Script/Engine.PlayerController|SetbEnableMouseOverEvents _returnvalue true)
  (Variables|/Script/Engine.PlayerController|SetbEnableClickEvents _returnvalue true))

(event Input|AxisEvents|InputAxisMouseX_Axis
  (params (AxisValue :type Float%20%28single-precision%29))
  ;[0 0 0] 鼠标控制镜头视角上下左右
  ;;[0.2969 0.2969 0.2969] 右键控制视角
  (if (Variables|Default|Get右键？)
    (Pawn|Input|AddControllerYawInput (Game|GetPlayerCharacter 0) AxisValue)))

(event Input|AxisEvents|InputAxisMouseY_Axis
  (params (AxisValue :type Float%20%28single-precision%29))
  ;[0 0 0] 鼠标控制镜头视角上下左右
  ;;[0.2969 0.2969 0.2969] 右键控制视角
  (if (Variables|Default|Get右键？)
    (Pawn|Input|AddControllerPitchInput (Game|GetPlayerCharacter 0) AxisValue)))

(event Input|AxisEvents|InputAxisLeft/Right
  (params (AxisValue :type Float%20%28single-precision%29))
  (bind _returnvalue (Pawn|GetControlRotation :!class /Script/Engine.Pawn))
  ;[0 0 0] WASD控制前后左右移动
  (Pawn|Input|AddMovementInput (Game|GetPlayerCharacter 0) (Math|Vector|GetRightVector (Math|Rotator|MakeRotator 0.0 (.pitch _returnvalue) (.yaw _returnvalue))) AxisValue false))

(event Input|AxisEvents|InputAxisUp/Down
  (params (AxisValue :type Float%20%28single-precision%29))
  (bind _returnvalue (Pawn|GetControlRotation :!class /Script/Engine.Pawn))
  ;[0 0 0] WASD控制前后左右移动
  (Pawn|Input|AddMovementInput (Game|GetPlayerCharacter 0) (Math|Vector|GetForwardVector (Math|Rotator|MakeRotator (.roll _returnvalue) 0.0 (.yaw _returnvalue))) AxisValue false))

(event Input|MouseEvents|RightMouseButton
  (params (Key :type Key%20Structure))
  ;[0 0 0] 鼠标控制镜头视角上下左右
  ;;[0.2865 0.2865 0.2865] 是否为鼠标右键
  (:Pressed
    (Variables|Default|Set右键？ true))
  (:Released
    (Variables|Default|Set右键？ false)))

(event Input|MouseEvents|LeftMouseButton
  (params (Key :type Key%20Structure))
  (bind _returnvalue (Viewport|GetViewportSize))
  (bind _returnvalue_2 (Game|GetPlayerController 0))
  (bind _returnvalue_3 (/ _returnvalue 2.0))
  (bind (_worldposition _worlddirection) (Class|GameplayStatics|DeprojectScreentoWorld _returnvalue_2 _returnvalue_3))
  (:Pressed
    (bind (_outhit _returnvalue_4) (Collision|LineTraceForObjects _worldposition (+ _worldposition (* _worlddirection 8e+02)) (Utilities|Array|MakeArray "ObjectTypeQuery4") false 0 "ForDuration")))
  (:Released
    (Physics|Components|PhysicsHandle|ReleaseComponent (Variables|Default|GetPhysicsHandle))
    (Variables|Default|SetHit%20Component 0)))

(fn ConstructionScript)

(fn 背包物品添加
  (params (添加物品 :type Medicine%20Info%20Structure))
  (bind _物品信息 (Variables|Default|Get物品信息))
  (Variables|Default|Set添加物品 添加物品)
  (bind _returnvalue (Utilities|Array|Add _物品信息 (Variables|Default|Get添加物品)))
  (Utilities|Array|SetArrayElem _物品信息 _returnvalue (Utilities|Struct|MakeMedicineInfo (.名称 (Utilities|Struct|BreakMedicineInfo (Variables|Default|Get添加物品))) (.模型 (Utilities|Struct|BreakMedicineInfo (Variables|Default|Get添加物品))) (.缩略图 (Utilities|Struct|BreakMedicineInfo (Variables|Default|Get添加物品))) (.药品种类 (Utilities|Struct|BreakMedicineInfo (Variables|Default|Get添加物品))) (.存放库区 (Utilities|Struct|BreakMedicineInfo (Variables|Default|Get添加物品))) _returnvalue)))