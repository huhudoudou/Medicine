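; Pawn Blueprint that provides hold-right-mouse-to-look camera input.
; The right mouse button sets a boolean while held, which gates the MouseX and MouseY axis events feeding controller yaw and pitch input.
; Left press, right press and right release each print a short Chinese debug label; left click does nothing else.
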(event Input|AxisEvents|InputAxisMouseX_Axis
  (params (AxisValue :type Float%20%28single-precision%29))
  (if (Variables|Default|Getif)
    (Pawn|Input|AddControllerYawInput AxisValue)))

(event Input|AxisEvents|InputAxisMouseY_Axis
  (params (AxisValue :type Float%20%28single-precision%29))
  (if (Variables|Default|Getif)
    (Pawn|Input|AddControllerPitchInput AxisValue)))

(event Input|MouseEvents|LeftMouseButton
  (params (Key :type Key%20Structure :default "None"))
  (:Pressed
    (Development|PrintText "左")))

(event Input|MouseEvents|RightMouseButton
  (params (Key :type Key%20Structure :default "None"))
  (:Pressed
    (Variables|Default|Setif true)
    (Development|PrintText "右"))
  (:Released
    (Variables|Default|Setif false)
    (Development|PrintText "冇")))

(fn ConstructionScript)